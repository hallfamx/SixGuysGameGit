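; Main menu game mode that shows the player's selected character at the BP_CharacterSpawn point.
; On BeginPlay it loads the Character save slot if present and copies the saved class into BP_GameInstance, otherwise it uses the game instance's current selection.
; It spawns that class at the first spawn actor found and keeps the reference.
; SpawnCharacter swaps the displayed character by destroying it and spawning the given class in its place.
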(event `self.ReceiveBeginPlay`
  (bind _asbp_game_instance (cast `/Game/UIX_System/Blueprints/GameInstance/BP_GameInstance` (`GameplayStatics.GetGameInstance`)))
  (set `self.GameInstance` _asbp_game_instance)
  (bind _returnvalue (`GameplayStatics.DoesSaveGameExist` "Character"))
  (if _returnvalue
    (bind _returnvalue_2 (`GameplayStatics.LoadGameFromSlot` "Character"))
    (bind _asbp_save_game (cast `/Game/UIX_System/Blueprints/Saves/BP_SaveGame` _returnvalue_2))
    (bind _selectedcharacter (`/Game/UIX_System/Blueprints/Saves/BP_SaveGame.SelectedCharacter` _asbp_save_game))
    (set `/Game/UIX_System/Blueprints/GameInstance/BP_GameInstance.SelectedCharacter` _selectedcharacter (`self.GameInstance`))
    (bind _outactors (`GameplayStatics.GetAllActorsOfClass` "/Game/UIX_System/Blueprints/Items/BP_CharacterSpawn.BP_CharacterSpawn_C"))
    (bind _returnvalue_3 (`|SpawnActorFromClass` _selectedcharacter (`self.GetTransform` (`|GetArrayItem` _outactors)) "Undefined" "OverrideRootScale" null null))
    (set `self.MainMenuCharacter` _returnvalue_3)
    (else
      (bind _outactors_2 (`GameplayStatics.GetAllActorsOfClass` "/Game/UIX_System/Blueprints/Items/BP_CharacterSpawn.BP_CharacterSpawn_C"))
      (bind _returnvalue_4 (`|SpawnActorFromClass` (`/Game/UIX_System/Blueprints/GameInstance/BP_GameInstance.SelectedCharacter` (`self.GameInstance`)) (`self.GetTransform` (`|GetArrayItem` _outactors_2)) "Undefined" "OverrideRootScale" null null))
      (set `self.MainMenuCharacter` _returnvalue_4))))

(event `SpawnCharacter`
  (params (CharacterClass :type "Character Class Reference"))
  (`self.K2_DestroyActor` (`self.MainMenuCharacter`))
  (bind _outactors (`GameplayStatics.GetAllActorsOfClass` "/Game/UIX_System/Blueprints/Items/BP_CharacterSpawn.BP_CharacterSpawn_C"))
  (bind _returnvalue (`|SpawnActorFromClass` CharacterClass (`self.GetTransform` (`|GetArrayItem` _outactors)) "Undefined" "OverrideRootScale" null null))
  (set `self.MainMenuCharacter` _returnvalue))

(fn `UserConstructionScript`)