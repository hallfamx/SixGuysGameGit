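; Lobby GameMode that manages connected players, lobby map settings, kicking and match start.
; Post-login registers each BP_LobbyController, creates its widget, then pushes map name, image and a rebuilt player list to every controller.
; Logout destroys the character and rebuilds lists, but only when that character is valid; kicking also clears the PlayerStart tag.
; Starting the game runs a servertravel console command to the map named by LobbyCode.
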(event `KickPlayer`
  (params (Index :type Integer))
  (bind _output (`|GetArrayItem` (`self.AllPlayers`) Index))
  ;[0 0 0] Kick Player - Destroy actor - Reset player start tag
  (`/Game/UIX_System/Blueprints/Controllers/BP_LobbyController.Kick` _output)
  (`self.K2_DestroyActor` (`/Game/UIX_System/Blueprints/Controllers/BP_LobbyController.PlayerCharacter` _output))
  (set `PlayerStart.PlayerStartTag` "None" (`/Game/UIX_System/Blueprints/Controllers/BP_LobbyController.PlayerStart` _output)))

(event `StartGame`
  ;[0 0 0] Start game
  (`KismetSystemLibrary.ExecuteConsoleCommand` (`KismetStringLibrary.Concat_StrStr` "servertravel /Game/Maps/" (`self.LobbyCode`)) null))

(event `Server Update Lobby Settings`
  (params (MapName :type String) (MapImage :type "Texture2D Object Reference"))
  ;[0 0 0] Server update lobby settings to all players
  (for _array_element (`self.AllPlayers`)
    (`/Game/UIX_System/Blueprints/Controllers/BP_LobbyController.Client Update Lobby Settings` _array_element MapName MapImage)))

(event `UpdateServer`
  ;[0 0 0] Update server - Clear playerlist - Add new player to list
  (for _array_element (`self.AllPlayers`)
    (`/Game/UIX_System/Blueprints/Controllers/BP_LobbyController.ClearPlayerList` _array_element)
    (for (_array_element_2 _array_index) (`self.AllPlayers`)
      (`/Game/UIX_System/Blueprints/Controllers/BP_LobbyController.AddPlayerToList` _array_element (`AdvancedSessionsLibrary.GetPlayerName` _array_element_2) _array_index))))

(event `self.K2_PostLogin`
  (params (NewPlayer :type "PlayerController Object Reference"))
  ;[0 0 0] OnPostLogin - Create lobby widget - Update lobby settings - Update server
  (bind _asbp_lobby_controller (cast `/Game/UIX_System/Blueprints/Controllers/BP_LobbyController` NewPlayer))
  (`KismetArrayLibrary.Array_Add` (`self.AllPlayers`) _asbp_lobby_controller)
  (`/Game/UIX_System/Blueprints/Controllers/BP_LobbyController.CreateLobbyWidget` _asbp_lobby_controller)
  (`self.Server Update Lobby Settings` (`self.LobbyMapName`) (`self.LobbyMapImage`))
  (`self.UpdateServer`))

(event `self.K2_OnLogout`
  (params (ExitingController :type "Controller Object Reference"))
  (bind _allplayers (`self.AllPlayers`))
  ;[0 0 0] OnLogout - Remove index - Update server
  (for (_array_element _array_index) _allplayers
    (if (== ExitingController _array_element)
      (break)))
  (bind _playercharacter (`/Game/UIX_System/Blueprints/Controllers/BP_LobbyController.PlayerCharacter` _array_element))
  (`/Engine/EditorBlueprintResources/StandardMacros.IsValid` _playercharacter
    (:`Is Valid`
      (`self.K2_DestroyActor` _playercharacter)
      (`KismetArrayLibrary.Array_Remove` _allplayers _array_index)
      (`self.UpdateServer`))))

(fn `UserConstructionScript`)