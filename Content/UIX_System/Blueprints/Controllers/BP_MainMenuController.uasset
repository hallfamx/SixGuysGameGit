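; Main menu player controller that sets up the menu UI and camera views and lets the mouse spin characters.
; BeginPlay destroys any session, cuts to the main camera and creates the CommonUI-style activatable menu widget.
; Events blend the view between main and customize cameras.
; A left-click trace selects a Character that Tick yaws by mouse delta; only pressing elsewhere clears it, as there is no release handler.
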(event `CreateMainMenuWidget`
  ;[0 0 0] Create main menu widget and show mouse cursor
  (bind _returnvalue (`|CreateWidget` "/Game/UIX_System/Widgets/WBP_MainMenu.WBP_MainMenu_C"))
  (bind _output_get (set `self.MainMenuWB` _returnvalue))
  (`UserWidget.AddToViewport` _output_get 0)
  (`CommonActivatableWidget.ActivateWidget` (`self.MainMenuWB`)))

(event `SetCustomzieCamera`
  ;[0 0 0] Set view target to customize camera
  (bind _outactors (`GameplayStatics.GetAllActorsOfClass` "/Game/UIX_System/Blueprints/Cameras/BP_CustomizeCamera.BP_CustomizeCamera_C"))
  (`self.SetViewTargetWithBlend` (`|GetArrayItem` _outactors) 0.5 "VTBlend_Linear" 0.0 true))

(event `SetStartingCamera`
  ;[0 0 0] Set view target to main menu camera
  (bind _outactors (`GameplayStatics.GetAllActorsOfClass` "/Game/UIX_System/Blueprints/Cameras/BP_MainCamera.BP_MainCamera_C"))
  (`self.SetViewTargetWithBlend` (`|GetArrayItem` _outactors) 0.0 "VTBlend_Linear" 0.0 true))

(event `SetMainMenuCamera`
  ;[0 0 0] Set view target to main menu camera
  (bind _outactors (`GameplayStatics.GetAllActorsOfClass` "/Game/UIX_System/Blueprints/Cameras/BP_MainCamera.BP_MainCamera_C"))
  (`self.SetViewTargetWithBlend` (`|GetArrayItem` _outactors) 0.5 "VTBlend_Linear" 0.0 true))

(event `self.ReceiveTick`
  (params (DeltaSeconds :type "Float (single-precision)"))
  ;[0 0 0] Rotate Character
  (`/Engine/EditorBlueprintResources/StandardMacros.IsValid` (stale `Key|LeftMouseButton` _output_get) :!label _label
    (:`Is Valid`
      (`self.K2_AddActorWorldRotation` (stale `Key|LeftMouseButton` _output_get) (`KismetMathLibrary.MakeRotator` 0.0 0.0 (* (`self.GetInputMouseDelta`) -50.0)) false false))))

(event `self.ReceiveBeginPlay`
  ;[0 0 0] BeginPlay - set main menu camera - create main menu widget
  (`DestroySessionCallbackProxy.DestroySession` self
    (:`then`
      (`self.SetStartingCamera`)
      (`self.CreateMainMenuWidget`))))

(event `Key|LeftMouseButton`
  (params (Key :type "Key Structure"))
  ;[0 0 0] Rotate Character
  (:`Pressed`
    (bind _ascharacter (cast `Character` (`.HitActor` (`GameplayStatics.BreakHitResult` (`self.GetHitResultUnderCursorByChannel` "TraceTypeQuery2"))))
      (:`then`
        (bind _output_get (set `self.RotateCharacter` _ascharacter))
        (goto _label))
      (:`CastFailed`
        (set `self.RotateCharacter` null)))))

(fn `UserConstructionScript`)