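; Player controller for gameplay that spawns the player's selected character and handles the pause menu and loading screen.
; On BeginPlay it reads the selected character from BP_GameInstance and passes it to a server event, then sets game-only input.
; The server tags the first untaken PlayerStart as "Taken", spawns the character there and possesses it.
; Pause input opens WBP_Pause with cursor and UI-only input, while a separate client event shows WBP_LoadingScreen.
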(event `self.ReceiveBeginPlay`
  ;[0 0 0] BeginPlay - Spawn character - Game only
  (`self.Client_SpawnCharacter`)
  (`WidgetBlueprintLibrary.SetInputMode_GameOnly` self))

(event `Client_LoadingScreen`
  ;[0 0 0] Loading screen
  (bind _returnvalue (`|CreateWidget` "/Game/UIX_System/Widgets/WBP_LoadingScreen.WBP_LoadingScreen_C"))
  (`UserWidget.AddToViewport` _returnvalue 0))

(event `Client_SpawnCharacter`
  ;[0 0 0] Client - Spawn Character
  (bind _asbp_game_instance (cast `/Game/UIX_System/Blueprints/GameInstance/BP_GameInstance` (`GameplayStatics.GetGameInstance`)))
  (`self.Server_SpawnCharacter` (`/Game/UIX_System/Blueprints/GameInstance/BP_GameInstance.SelectedCharacter` _asbp_game_instance)))

(event `InputAction|Pause`
  (params (Key :type "Key Structure"))
  ;[0 0 0] Pause - Create widget - Add to viewport - UI only
  (:`Pressed`
    (bind _returnvalue (`|CreateWidget` "/Game/UIX_System/Widgets/WBP_Pause.WBP_Pause_C"))
    (`UserWidget.AddToViewport` _returnvalue 0)
    (set `self.bShowMouseCursor` true)
    (`WidgetBlueprintLibrary.SetInputMode_UIOnlyEx` self _returnvalue)))

(event `Server_SpawnCharacter`
  (params (CharacterToSpawn :type "Character Class Reference"))
  ;[0 0 0] Server - Spawn Character
  (bind _outactors (`GameplayStatics.GetAllActorsOfClass` "/Script/Engine.PlayerStart"))
  (for _array_element _outactors
    (if (!= (`PlayerStart.PlayerStartTag` _array_element) "Taken")
      (set `PlayerStart.PlayerStartTag` "Taken" _array_element)
      (break)))
  (bind _returnvalue (`|SpawnActorFromClass` CharacterToSpawn (`self.GetTransform` _array_element) "Undefined" "OverrideRootScale" null null))
  (`self.Possess` self _returnvalue))

(fn `UserConstructionScript`)