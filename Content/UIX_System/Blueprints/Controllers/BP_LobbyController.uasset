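; Lobby player controller that manages each player's lobby widget, camera view and display character in a multiplayer lobby.
; On BeginPlay it switches view to the lobby camera and passes the GameInstance's selected character to a server spawn event.
; That event tags a free PlayerStart as taken and spawns a fixed parkour character there, ignoring the selection.
; Other events update map info and player list, show a loading screen, and handle kicks by destroying the session.
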(event `Client Update Lobby Settings`
  (params (MapName :type String) (MapImage :type "Texture2D Object Reference"))
  (bind _lobbywb (`self.LobbyWB`))
  ;[0 0 0] Client update lobby settings
  (set `/Game/UIX_System/Widgets/WBP_Lobby.LobbyMapImage` MapImage _lobbywb)
  (set `/Game/UIX_System/Widgets/WBP_Lobby.LobbyMapName` MapName _lobbywb))

(event `ClearPlayerList`
  ;[0 0 0] Clear playerlist - Add player to list
  (`/Game/UIX_System/Widgets/WBP_Lobby.ClearPlayerList` (`self.LobbyWB`)))

(event `CreateLobbyWidget`
  ;[0 0 0] Create lobby widget
  (bind _returnvalue (`|CreateWidget` "/Game/UIX_System/Widgets/WBP_Lobby.WBP_Lobby_C" null "" null))
  (bind _output_get (set `self.LobbyWB` _returnvalue))
  (`UserWidget.AddToViewport` _output_get 0)
  (set `self.bShowMouseCursor` true)
  (`WidgetBlueprintLibrary.SetInputMode_UIOnlyEx` self _output_get))

(event `AddPlayerToList`
  (params (PlayerName :type String) (PlayerIndex :type Integer))
  ;[0 0 0] Clear playerlist - Add player to list
  (`/Game/UIX_System/Widgets/WBP_Lobby.AddPlayerToList` (`self.LobbyWB`) PlayerName PlayerIndex))

(event `Client_SpawnCharacter`
  ;[0 0 0] Client - Spawn Character
  (bind _asbp_game_instance (cast `/Game/UIX_System/Blueprints/GameInstance/BP_GameInstance` (`GameplayStatics.GetGameInstance`)))
  (`self.Server_SpawnCharacter` (`/Game/UIX_System/Blueprints/GameInstance/BP_GameInstance.SelectedCharacter` _asbp_game_instance)))

(event `SetLobbyCamera`
  ;[0 0 0] Set view target to lobby camera
  (bind _outactors (`GameplayStatics.GetAllActorsOfClass` "/Game/UIX_System/Blueprints/Cameras/BP_LobbyCamera.BP_LobbyCamera_C"))
  (`self.SetViewTargetWithBlend` (`|GetArrayItem` _outactors)))

(event `Client_LoadingScreen`
  ;[0 0 0] Loading screen
  (bind _returnvalue (`|CreateWidget` "/Game/UIX_System/Widgets/WBP_LoadingScreen.WBP_LoadingScreen_C"))
  (`UserWidget.AddToViewport` _returnvalue 0))

(event `Server_SpawnCharacter`
  (params (CharacterToSpawn :type "Character Class Reference"))
  ;[0 0 0] Server - Spawn Character
  (bind _outactors (`GameplayStatics.GetAllActorsOfClass` "/Script/Engine.PlayerStart"))
  (for _array_element _outactors
    (if (!= (`PlayerStart.PlayerStartTag` _array_element) "Taken")
      (set `PlayerStart.PlayerStartTag` "Taken" _array_element)
      (set `self.PlayerStart` _array_element)
      (break)))
  (bind _returnvalue (`|SpawnActorFromClass` "/Game/PlayerCharacter/BluePrints/BP_FPParkourChar_MP.BP_FPParkourChar_MP_C" (`self.GetTransform` _array_element) "Undefined" "OverrideRootScale" null null))
  (set `self.PlayerCharacter` _returnvalue))

(event `self.ReceiveBeginPlay`
  ;[0 0 0] BeginPlay - Set lobby camera - Spawn character
  (`self.SetLobbyCamera`)
  (`self.Client_SpawnCharacter`))

(event `Kick`
  ;[0 0 0] Kick player
  (`DestroySessionCallbackProxy.DestroySession` self
    (:`then`
      (`GameplayStatics.OpenLevel` "MainMenu"))))

(fn `UserConstructionScript`)