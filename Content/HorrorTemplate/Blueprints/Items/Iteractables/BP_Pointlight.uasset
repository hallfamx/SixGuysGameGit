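; BP_Pointlight is an interactable point light for the horror template that the Use event toggles on and off.
; The construction script applies exposed mesh, light and shadow settings, plus the starting on or off state.
; Use flips the light's visibility and swaps the mesh between on and off materials to match.
; When ShouldFlicker is set, a timeline started on BeginPlay drives intensity on a hardcoded 5000 scale, overriding the configured Intensity.
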(event `self.Use`
  (params (MiscUse1 :type Boolean))
  (bind _pointlight (`self.PointLight`))
  (`SceneComponent.ToggleVisibility` _pointlight false)
  (if (`SceneComponent.IsVisible` _pointlight)
    ;[1 1 1] Set on and off material
    (`PrimitiveComponent.SetMaterial` (`self.StaticMesh`) 0 (`self.OnMaterial`))
    (else
      (`PrimitiveComponent.SetMaterial` (`self.StaticMesh`) 0 (`self.OffMaterial`)))))

(event `self.ReceiveBeginPlay`
  ;[1 1 1] If should flicker, play timeline that changes light intensity
  (if (`self.ShouldFlicker`)
    (bind (_direction _newtrack_0) (`Timeline|Flicker`)
      (:`Update`
        (`LightComponent.SetIntensity` (`self.PointLight`) (* _newtrack_0 5000.0))))))

(fn `UserConstructionScript`
  (bind _pointlight (`self.PointLight`))
  ;[1 1 1] Set light parameters
  (`StaticMeshComponent.SetStaticMesh` (`self.StaticMesh`) (`self.Mesh`))
  (`SceneComponent.SetVisibility` _pointlight (`self.StartEnabled`) false)
  (`LightComponent.SetIntensity` _pointlight (`self.Intensity`))
  (`LightComponent.SetLightColor` _pointlight (`self.Colour`) true)
  (`PointLightComponent.SetAttenuationRadius` _pointlight (`self.AttenuationRadius`))
  (`PointLightComponent.SetSourceRadius` _pointlight (`self.SourceRadius`))
  (`PointLightComponent.SetSourceLength` _pointlight (`self.SourceLength`))
  (`LightComponentBase.SetCastShadows` _pointlight (`self.CastShadows`))
  (if (`self.StartEnabled`)
    (`PrimitiveComponent.SetMaterial` (`self.StaticMesh`) 0 (`self.OnMaterial`))
    (else
      (`PrimitiveComponent.SetMaterial` (`self.StaticMesh`) 0 (`self.OffMaterial`)))))