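; BP_Button is a usable button that triggers Use on linked interactable actors, optionally unlocking them or firing only once.
; Each successful trigger plays a sound and optional motion: a skeletal animation, or timeline-driven rotation or movement.
; FlipFlops alternate timeline direction, with an optional delayed return.
; The construction script assigns meshes, sets timeline speed and hides whichever mesh the animation mode leaves unused.
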(event `self.Use`
  (params (MiscUse1 :type Boolean))
  (bind _returnvalue (`self.K2_GetActorLocation` self))
  ;[1 1 1] If button is to only be used once, and has fired then dont use again
  (if (`self.FireOnce`)
    (if (not (`self.HasFired`))
      ;[1 1 1] Loop for all added actors
      (for _array_element (`self.OtherActor`) :!label _label
        (bind _asbp_interactable (cast `/Game/HorrorTemplate/Blueprints/Items/Iteractables/BP_Interactable` _array_element)
          (:`then`
            ;[1 1 1] Should the button unlock something on use?
            (`self.Use` _asbp_interactable (`self.ShouldUnlock`))
            (set `self.HasFired` true)
            ;[1 1 1] Play use sound
            (`GameplayStatics.PlaySoundAtLocation` (`self.UseSound`) (`self.K2_GetActorLocation` self) (struct) 1.0 1.0 0.0 null null null null)
            ;[1 1 1] Determine if should move or animate on use
            (if (`self.ShouldMoveOnUse`)
              (if (`self.ShouldAnimate`)
                ;[1 1 1] Play a skeletal animation rather than manually moving object
                (`SkeletalMeshComponent.PlayAnimation` (`self.SkeletalMesh`) (`self.UseAnimation`) false)
                (elif (`self.ShouldRotate`)
                  ;[1 1 1] Rotate
                  (`/Engine/EditorBlueprintResources/StandardMacros.FlipFlop`
                    (:`A`
                      (bind (_direction _movealpha) (`Timeline|Rotate` :!label _label_2)
                        (:`Update`
                          (`SceneComponent.K2_SetRelativeRotation` (`self.Origin`) (`KismetMathLibrary.RLerp` (struct) (`self.RotationAngle`) _movealpha) false false)
                          (if (`self.ShouldReturnToInitialState`)
                            (`KismetSystemLibrary.Delay` (`self.ReturnInitialStateTime`))
                            (goto _label_2 :!via `Reverse`)))))
                    (:`B`
                      (goto _label_2 :!via `Reverse`)))
                  (else
                    ;[1 1 1] Move
                    (`/Engine/EditorBlueprintResources/StandardMacros.FlipFlop`
                      (:`A`
                        (bind (_direction_2 _movealpha_2) (`Timeline|Move` :!label _label_3)
                          (:`Update`
                            (`SceneComponent.K2_SetWorldLocation` (`self.StaticMesh`) (`KismetMathLibrary.VLerp` _returnvalue (+ _returnvalue (`self.MoveDistance`)) _movealpha_2) false false)
                            (if (`self.ShouldReturnToInitialState`)
                              (`KismetSystemLibrary.Delay` (`self.ReturnInitialStateTime`))
                              (goto _label_3 :!via `Reverse`)))))
                      (:`B`
                        (goto _label_3 :!via `Reverse`))))))))
          (:`CastFailed`
            ;[1 1 1] Fail Event
            (`KismetSystemLibrary.PrintString` "INTERACTABLE CAST FALED" true true (struct :`R` 1.0 :`A` 1.0))))))
    (else
      (goto _label))))

(fn `UserConstructionScript`
  (bind _movespeed (`self.MoveSpeed`))
  (`parent.UserConstructionScript`)
  (`SkinnedMeshComponent.SetSkinnedAssetAndUpdate` (`self.SkeletalMesh`) (`self.Animated Button Mesh`) true)
  (`StaticMeshComponent.SetStaticMesh` (`self.StaticMesh`) (`self.Button Mesh`))
  ;[1 1 1] Set speed of move/rotation
  (`TimelineComponent.SetPlayRate` (`self.Move`) _movespeed)
  (`TimelineComponent.SetPlayRate` (`self.Rotate`) _movespeed)
  (if (`self.ShouldAnimate`)
    (`SceneComponent.SetVisibility` (`self.StaticMesh`) false false)
    (else
      (`SceneComponent.SetVisibility` (`self.SkeletalMesh`) false false))))