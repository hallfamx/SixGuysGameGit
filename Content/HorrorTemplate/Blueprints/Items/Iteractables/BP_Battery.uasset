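; Battery pickup interactable for the horror template that recharges the player's flashlight when used.
; Use casts player 0 to HorrorTemplateCharacter and adds EnergyAmount to FlashlightEnergy, capped at 100, or only prints a message if already full.
; It also raises FlashlightIntensity in proportion to the full EnergyAmount, even when energy is capped, then plays a pickup sound and destroys itself.
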(event `self.Use`
  (params (MiscUse1 :type Boolean))
  ;[1 1 1] Cast to player to get flashlight values
  (bind _ashorror_template_character (cast `/Game/HorrorTemplate/Blueprints/Character/HorrorTemplateCharacter` (`GameplayStatics.GetPlayerCharacter` 0))
    (:`then`
      (bind _flashlightenergy (`/Game/HorrorTemplate/Blueprints/Character/HorrorTemplateCharacter.FlashlightEnergy` _ashorror_template_character))
      ;[1 1 1] If flashlight is at 100%, dont give it any more energy
      (if (>= _flashlightenergy 100.0)
        (`KismetSystemLibrary.PrintString` "Battery Full!" true true (struct :`R` 0.818464 :`G` 1.0 :`B` 0.090821 :`A` 1.0))
        (else
          (if (not (< (- 100.0 _flashlightenergy) (`self.EnergyAmount`)))
            ;[1 1 1] Add both given and existing energy together
            (set `/Game/HorrorTemplate/Blueprints/Character/HorrorTemplateCharacter.FlashlightEnergy` (+ (`/Game/HorrorTemplate/Blueprints/Character/HorrorTemplateCharacter.FlashlightEnergy` _ashorror_template_character) (`self.EnergyAmount`)) _ashorror_template_character)
            (else
              ;[1 1 1] Otherwise just set energy to max
              (set `/Game/HorrorTemplate/Blueprints/Character/HorrorTemplateCharacter.FlashlightEnergy` 100.0 _ashorror_template_character)))
          (set `/Game/HorrorTemplate/Blueprints/Character/HorrorTemplateCharacter.FlashlightIntensity` (+ (* (/ (`self.EnergyAmount`) 100.0) 5000.0) (`/Game/HorrorTemplate/Blueprints/Character/HorrorTemplateCharacter.FlashlightIntensity` _ashorror_template_character)) _ashorror_template_character)
          (`GameplayStatics.PlaySound2D` (`self.PickupSound`) 0.25 1.0 0.0 null null)
          (`self.K2_DestroyActor`))))
    (:`CastFailed`
      ;[1 1 1] Fail Event
      (`KismetSystemLibrary.PrintString` "PLAYER CAST FALED" true true (struct :`R` 1.0 :`A` 1.0)))))

(fn `UserConstructionScript`
  (`parent.UserConstructionScript`))