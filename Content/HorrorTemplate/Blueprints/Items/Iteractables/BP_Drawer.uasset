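; BP_Drawer is an interactable drawer that slides open and closed when used.
; Each Use alternates between playing and reversing a timeline, which lerps the Drawer mesh's relative location from zero along its Y axis by the negated MoveDistance.
; The construction script calls the parent's, assigns the configurable mesh and sets the timeline play rate to the inverse of OpenSpeed, so that value acts as a duration scale.
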(event `self.Use`
  (params (MiscUse1 :type Boolean))
  ;[1 1 1] Open drawer move distance
  (`/Engine/EditorBlueprintResources/StandardMacros.FlipFlop`
    (:`A`
      (bind (_direction _delta) (`Timeline|DrawerTimeline` :!label _label)
        (:`Update`
          (`SceneComponent.K2_SetRelativeLocation` (`self.Drawer`) (`KismetMathLibrary.VLerp` (0.0 0.0 0.0) (`KismetMathLibrary.MakeVector` 0.0 (* (`self.MoveDistance`) -1.0)) _delta) false false))))
    (:`B`
      (goto _label :!via `Reverse`))))

(fn `UserConstructionScript`
  (`parent.UserConstructionScript`)
  (`StaticMeshComponent.SetStaticMesh` (`self.Drawer`) (`self.Mesh`))
  (`TimelineComponent.SetPlayRate` (`self.DrawerTimeline`) (/ 1.0 (`self.OpenSpeed`))))