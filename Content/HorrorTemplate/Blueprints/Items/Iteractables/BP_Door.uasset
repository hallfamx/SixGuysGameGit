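; Interactable hinged door for the horror template that swings open or closed on each Use, or plays a locked sound.
; A true MiscUse1 input bypasses the Locked check.
; A FlipFlop plays or reverses a timeline that yaws the hinge forward or backward by a configurable amount, with attached sounds.
; Construction sets mesh, speed and initial rotation, which gates the stop sound when a second FlipFlop marks the door closed.
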(event `self.Use`
  (params (MiscUse1 :type Boolean))
  (bind _hinge (`self.Hinge`))
  (if MiscUse1
    (`/Engine/EditorBlueprintResources/StandardMacros.FlipFlop` :!label _label
      (:`A`
        ;[1 1 1] Play open sound
        (`GameplayStatics.SpawnSoundAttached` (`self.DoorOpenSound`) (`self.Door`) "None" (0.0 0.0 0.0) (struct) "KeepRelativeOffset" false (`self.DoorOpenSoundVolume`) 1.0 0.0 (`self.DoorAttenuation`) null)
        ;[1 1 1] Open door animation
        (bind (_direction _openangle) (`Timeline|DoorTimeLine` :`NewTime` 0.0 :!label _label_2)
          (:`Update`
            (set `self.IsOpening` true)
            (if (`self.OpenForward`)
              (bind _returnvalue (`KismetMathLibrary.MakeRotator` 0.0 0.0 (`KismetMathLibrary.MapRangeClamped` _openangle 0.0 90.0 0.0 (`self.Open Amount`))))
              ;[1 1 1] Either open forward or backwards
              (`SceneComponent.K2_SetRelativeRotation` _hinge _returnvalue true false)
              (else
                (`SceneComponent.K2_SetRelativeRotation` _hinge (* _returnvalue -1) true false))))
          (:`Finished`
            (`/Engine/EditorBlueprintResources/StandardMacros.FlipFlop`
              (:`A`
                (set `self.Closed` false))
              (:`B`
                (set `self.Closed` true)
                (if (== (`SceneComponent.RelativeRotation` (`self.Hinge`)) (`self.InitialDoorRotation`) :`ErrorTolerance` 1.0)
                  ;[1 1 1] Play stop sound
                  (`GameplayStatics.SpawnSoundAttached` (`self.DoorStopSound`) (`self.Door`) "None" (0.0 0.0 0.0) (struct) "KeepRelativeOffset" false (`self.DoorStopSoundVolume`) 1.0 0.0 (`self.DoorAttenuation`) null)
                  (set `self.IsOpening` false)))))))
      (:`B`
        (`GameplayStatics.SpawnSoundAttached` (`self.DoorOpenSound`) (`self.Door`) "None" (0.0 0.0 0.0) (struct) "KeepRelativeOffset" false (`self.DoorOpenSoundVolume`) 1.0 0.0 (`self.DoorAttenuation`) null)
        (goto _label_2 :!via `Reverse`)))
    (else
      ;[1 1 1] If door is locked then play a sound
      (if (`self.Locked`)
        (`GameplayStatics.SpawnSoundAttached` (`self.DoorLockedSound`) (`self.Door`) "None" (0.0 0.0 0.0) (struct) "KeepRelativeOffset" false (`self.DoorLockedSoundVolume`) 1.0 0.0 (`self.DoorAttenuation`) null)
        (else
          (goto _label))))))

(fn `UserConstructionScript`
  ;[1 1 1] Set mesh
  (`StaticMeshComponent.SetStaticMesh` (`self.Door`) (`self.DoorMesh`))
  (`TimelineComponent.SetPlayRate` (`self.DoorTimeLine`) (`self.Open Speed`))
  ;[1 1 1] Remember the doors initial rotation
  (set `self.InitialDoorRotation` (`SceneComponent.RelativeRotation` (`self.Door`))))