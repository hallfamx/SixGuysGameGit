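; BP_glowstick is a glowstick prop with a static mesh and a point light, configurable per instance.
; The Construction Script creates a dynamic material from Mat_glowstick and feeds it the colour and glow strength.
; The same colour drives the point light, alongside exposed intensity, attenuation, shadow and visibility settings, while mesh shadow casting is disabled.
; The Event Graph holds no runtime logic.
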(event `self.ReceiveTick`
  (params (DeltaSeconds :type "Float (single-precision)")))

(fn `UserConstructionScript`
  (bind _colour (`self.Colour`))
  (bind _pointlight (`self.PointLight`))
  (bind _returnvalue (`PrimitiveComponent.CreateDynamicMaterialInstance` (`self.StaticMesh`) 0 "/Game/HorrorTemplate/Materials/Items/mat_glowstick.mat_glowstick" "None"))
  ;[1 1 1] Set light parameters
  (`MaterialInstanceDynamic.SetVectorParameterValue` _returnvalue "Color" _colour)
  (`MaterialInstanceDynamic.SetScalarParameterValue` _returnvalue "GlowStrength" (`self.GlowStrength`))
  (`LightComponent.SetLightColor` (`self.PointLight`) _colour true)
  (`LightComponent.SetIntensity` _pointlight (`self.Intensity`))
  (`PointLightComponent.SetAttenuationRadius` _pointlight (`self.Attenuation`))
  (`LightComponentBase.SetCastShadows` _pointlight (`self.CastShadows`))
  (`SceneComponent.SetVisibility` _pointlight (`self.Visibility`) false)
  (`PrimitiveComponent.SetCastShadow` (`self.StaticMesh`) false))