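; Game instance that manages multiplayer sessions and the game's menu and HUD widgets.
; It creates sessions by opening a listen-server level, fills the Find Session widget with slots from search results, and destroys the session to return to the menu level.
; Show events lazily create and cache each widget, then a shared WidgetCheck sets visibility, cursor and input mode.
; DetectWidgetChange swaps out the current main screen, while pause and settings bypass it.
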(event `Event Create Session`
  (params (PlayerController :type "PlayerController Object Reference") (PublicConnections :type Integer) (bUseLAN :type Boolean) (Level :type "World Soft Object Reference"))
  (`CreateSessionCallbackProxy.CreateSession` PlayerController PublicConnections bUseLAN
    (:`OnSuccess`
      (bind _output_get (set `self.Level` Level))
      (`GameplayStatics.OpenLevelBySoftObjectPtr` _output_get true "Listen"))))

(event `Event Find Sessions`
  (params (PlayerController :type "PlayerController Object Reference") (MaxResults :type Integer) (bUseLAN :type Boolean))
  (bind _findsession_wbp_ref (`self.FindSession WBP Ref`))
  (bind _scrollbox_0 (`/Game/Multiplayer/Core/Blueprints/UI/Widgets/Menus/FindSession_WBP.ScrollBox_0` _findsession_wbp_ref))
  (bind _circularthrobber_0 (`/Game/Multiplayer/Core/Blueprints/UI/Widgets/Menus/FindSession_WBP.CircularThrobber_0` _findsession_wbp_ref))
  (bind _searchbutton (`/Game/Multiplayer/Core/Blueprints/UI/Widgets/Menus/FindSession_WBP.SearchButton` _findsession_wbp_ref))
  (`PanelWidget.ClearChildren` _scrollbox_0)
  (`Widget.SetVisibility` _circularthrobber_0 "Visible")
  (`Widget.SetIsEnabled` _searchbutton false)
  (bind _results (`FindSessionsCallbackProxy.FindSessions` PlayerController MaxResults bUseLAN)
    (:`then`
      (for _array_element _results
        (bind _returnvalue (`|CreateWidget` "/Game/Multiplayer/Core/Blueprints/UI/Widgets/Menus/SessionSlot_WBP.SessionSlot_WBP_C" PlayerController _array_element))
        (bind _output_get (set `self.Session Slot WBP Ref` _returnvalue))
        (`UserWidget.AddToViewport` _output_get 0)
        (`PanelWidget.AddChild` _scrollbox_0 _output_get))
      (`KismetSystemLibrary.Delay` 0.5)
      (`Widget.SetVisibility` _circularthrobber_0 "Hidden")
      (`Widget.SetIsEnabled` _searchbutton true))))

(event `Event Leave Game`
  (params (PlayerController :type "PlayerController Object Reference"))
  (`DestroySessionCallbackProxy.DestroySession` PlayerController
    (:`OnSuccess`
      (`GameplayStatics.OpenLevelBySoftObjectPtr` "/Game/Multiplayer/Core/Worlds/Levels/MultiplayerMenu_Level.MultiplayerMenu_Level"))))

(event `Event Widget Check`
  (params (`Player Controller Referance` :type "PlayerController Object Reference") (`Widget Referance` :type "UserWidget Object Reference") (ZOrder :type Integer) (Visibility :type "ESlateVisibility Enum" :default "Visible") (`InGameCall?` :type Boolean) (`Show Mouse?` :type Boolean) (`0=GameOnly | 1=UIOnly | 2=Both` :type Integer :default 1))
  (if (not `InGameCall?`)
    (if (not (`Widget.IsVisible` `Widget Referance`))
      (`Widget.SetVisibility` `Widget Referance` Visibility))
    (if (not (`Widget.IsInViewport` `Widget Referance`))
      (`UserWidget.AddToViewport` `Widget Referance` ZOrder)))
  (if `Show Mouse?`
    (set `PlayerController.bShowMouseCursor` true `Player Controller Referance`)
    (else
      (set `PlayerController.bShowMouseCursor` false `Player Controller Referance`)))
  (if `InGameCall?`
    (`WidgetBlueprintLibrary.SetInputMode_GameOnly` `Player Controller Referance` :!label _label)
    (else
      (switch `int` `0=GameOnly | 1=UIOnly | 2=Both`
        (:`0`
          (goto _label))
        (:`1`
          (`WidgetBlueprintLibrary.SetInputMode_UIOnlyEx` `Player Controller Referance` `Widget Referance` "LockOnCapture"))
        (:`2`
          (`WidgetBlueprintLibrary.SetInputMode_GameAndUIEx` `Player Controller Referance` `Widget Referance` "LockOnCapture" false))))))

(event `Show MainMenu Widget`
  (params (Controller :type "PlayerController Object Reference"))
  (`/Engine/EditorBlueprintResources/StandardMacros.IsValid` (`self.MainMenu WBP Ref`)
    (:`Is Valid`
      _)
    (:`Is Not Valid`
      (bind _returnvalue (`|CreateWidget` "/Game/Multiplayer/Core/Blueprints/UI/Widgets/Menus/MainMenu_WBP.MainMenu_WBP_C" Controller))
      (bind _output_get (set `self.MainMenu WBP Ref` _returnvalue))))
  (bind _output_widget (`self.Detect Widget Change` _output_get))
  (`self.Event Widget Check` Controller _output_widget 1 "Visible" false true))

(event `Show Pause Widget`
  (params (Controller :type "PlayerController Object Reference"))
  (`/Engine/EditorBlueprintResources/StandardMacros.IsValid` (`self.PauseMenu WBP Ref`)
    (:`Is Valid`
      _)
    (:`Is Not Valid`
      (bind _returnvalue (`|CreateWidget` "/Game/Multiplayer/Core/Blueprints/UI/Widgets/InGame/PauseMenu_WBP.PauseMenu_WBP_C" Controller))
      (bind _output_get (set `self.PauseMenu WBP Ref` _returnvalue))))
  (`self.Event Widget Check` Controller _output_get 2 "Visible" false true 2))

(event `Show Settings Widget`
  (params (Controller :type "PlayerController Object Reference"))
  (`/Engine/EditorBlueprintResources/StandardMacros.IsValid` (`self.Settings WBP Ref`)
    (:`Is Valid`
      _)
    (:`Is Not Valid`
      (bind _returnvalue (`|CreateWidget` "/Game/Multiplayer/Core/Blueprints/UI/Widgets/Menus/SettingsMenu_WBP.SettingsMenu_WBP_C" Controller))
      (bind _output_get (set `self.Settings WBP Ref` _returnvalue))))
  (`self.Event Widget Check` Controller _output_get 3 "Visible" false true))

(event `Show HUD Widget`
  (params (Controller :type "PlayerController Object Reference"))
  (`/Engine/EditorBlueprintResources/StandardMacros.IsValid` (`self.HUD WBP Ref`)
    (:`Is Valid`
      _)
    (:`Is Not Valid`
      (bind _returnvalue (`|CreateWidget` "/Game/Multiplayer/Core/Blueprints/UI/Widgets/InGame/HUD_WBP.HUD_WBP_C" Controller))
      (bind _output_get (set `self.HUD WBP Ref` _returnvalue))))
  (bind _output_widget (`self.Detect Widget Change` _output_get))
  (`self.Event Widget Check` Controller _output_widget 1 "Visible" false false 0))

(event `Show Create Session Widget`
  (params (Controller :type "PlayerController Object Reference"))
  (`/Engine/EditorBlueprintResources/StandardMacros.IsValid` (`self.CreateSession WBP Ref`)
    (:`Is Valid`
      _)
    (:`Is Not Valid`
      (bind _returnvalue (`|CreateWidget` "/Game/Multiplayer/Core/Blueprints/UI/Widgets/Menus/CreateSession_WBP.CreateSession_WBP_C" Controller))
      (bind _output_get (set `self.CreateSession WBP Ref` _returnvalue))))
  (bind _output_widget (`self.Detect Widget Change` _output_get))
  (`self.Event Widget Check` Controller _output_widget 1 "Visible" false true))

(event `Show Find Session Widget`
  (params (Controller :type "PlayerController Object Reference"))
  (`/Engine/EditorBlueprintResources/StandardMacros.IsValid` (`self.FindSession WBP Ref`)
    (:`Is Valid`
      _)
    (:`Is Not Valid`
      (bind _returnvalue (`|CreateWidget` "/Game/Multiplayer/Core/Blueprints/UI/Widgets/Menus/FindSession_WBP.FindSession_WBP_C" Controller))
      (bind _output_get (set `self.FindSession WBP Ref` _returnvalue))))
  (bind _output_widget (`self.Detect Widget Change` _output_get))
  (`self.Event Widget Check` Controller _output_widget 1 "Visible" false true))

(fn `Detect Widget Change`
  (params (`Input Widget` :type "UserWidget Object Reference"))
  (returns (`Output Widget` :type "UserWidget Object Reference"))
  (bind _current_widget (`self.Current Widget`))
  (if (not (== `Input Widget` _current_widget))
    (if (not (== _current_widget null))
      (`Widget.RemoveFromParent` _current_widget))
    (bind _output_get (set `self.Current Widget` `Input Widget`)))
  (return _output_get))