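; GM_Shooter, apparently a shooter game mode by its name, picks random respawn transforms from the level's PlayerStart actors.
; CalculateSpawnLocation returns a random SpawnPoints entry, filling that array through GetAllActorsOfClass when the sampled entry is invalid.
; The validity check and the return each roll their own random index, so they can hit different entries.
; CheckForGameOver and the construction script are empty.
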(fn `CalculateSpawnLocation`
  (returns (SpawnLocation :type "Transform Structure"))
  (locals (PlayerToSpawnOn :type Boolean))
  (bind _spawnpoints (`self.SpawnPoints`))
  (bind _output (`|GetArrayItem` _spawnpoints (`KismetMathLibrary.RandomIntegerInRange` 0 (- (`KismetArrayLibrary.Array_Length` _spawnpoints) 1))))
  ;[1 1 1] Use Spawn Points to Respawn On
  (`/Engine/EditorBlueprintResources/StandardMacros.IsValid` _output
    (:`Is Valid`
      (return (`self.GetTransform` _output)))
    (:`Is Not Valid`
      (bind _outactors (`GameplayStatics.GetAllActorsOfClass` "/Script/Engine.PlayerStart")) ; Get All Player Spawn Points
      (bind _output_get (set `self.SpawnPoints` _outactors))
      (return (`self.GetTransform` (`|GetArrayItem` _output_get (`KismetMathLibrary.RandomIntegerInRange` 0 (- (`KismetArrayLibrary.Array_Length` _output_get) 1))))))))

(fn `CheckForGameOver`)

(fn `UserConstructionScript`)