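; Animation notify that plays surface-dependent footstep sounds for the character whose mesh triggers it.
; It sends a FootstepMessage to the owning actor, then traces 150 units down from the owner's root on the Visibility channel.
; The hit's physical surface picks the sand cue or, for concrete and anything else, the default cue, played at the impact point with footstep attenuation.
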(fn `GetLocation`
  (returns (CharacterLocation :type "Vector Structure"))
  (return (0.0 0.0 0.0)))

(fn `Is Player?`
  (returns (`Yes/No` :type Boolean))
  (return false))

(fn `Received_Notify`
  (params (MeshComp :type "SkeletalMeshComponent Object Reference") (Animation :type "AnimSequenceBase Object Reference") (EventReference :type "AnimNotifyEventReference Structure (by ref)"))
  (returns (ReturnValue :type Boolean))
  (bind _returnvalue (`ActorComponent.GetOwner` MeshComp))
  (bind _returnvalue_2 (`SceneComponent.K2_GetComponentLocation` (`Actor.RootComponent` _returnvalue)))
  (message `/Game/PlayerCharacter/BluePrints/BPI_PlayerCharacter.Footstep` _returnvalue)
  (bind (_outhit _returnvalue_3) (`KismetSystemLibrary.LineTraceSingle` _returnvalue_2 (- _returnvalue_2 (0.0 0.0 150.0)) "TraceTypeQuery1"))
  (if _returnvalue_3
    (switch `EPhysicalSurface` (`GameplayStatics.GetSurfaceType` _outhit)
      (:`SurfaceType_Default`
        (bind (_bblockinghit _binitialoverlap _time _distance _location) (`GameplayStatics.BreakHitResult` _outhit))
        (`GameplayStatics.SpawnSoundAtLocation` "/Game/PlayerCharacter/Sounds/FootStepsCues/Default_Footstep_Cue.Default_Footstep_Cue" _location (struct) 0.8 1.0 0.0 "/Game/PlayerCharacter/Sounds/Footstep_Attenuation.Footstep_Attenuation" null :!label _label)
        (return false))
      (:`SurfaceType1`
        (goto _label))
      (:`SurfaceType2`
        (`GameplayStatics.SpawnSoundAtLocation` "/Game/PlayerCharacter/Sounds/FootStepsCues/Sand_Footstep_Cue.Sand_Footstep_Cue" _location (struct) 0.6 1.0 0.0 "/Game/PlayerCharacter/Sounds/Footstep_Attenuation.Footstep_Attenuation" null)))))