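; BP_IceCloud is a player spell actor that creates a timed area-of-effect ice cloud.
; A sphere overlap sends IceStormMessage with damage, duration and an IceCloud flag to actors implementing HealthDamageInterface, excluding the instigator.
; Sound fades in on spawn; after Duration, the Niagara effect deactivates and sound fades out.
; Niagara's deactivation event then turns off the sphere and destroys the actor after a delay.
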(event `self.ReceiveBeginPlay`
  (bind _spellsound (`self.SpellSound`))
  (set `self.AttackingActor` (`self.GetInstigator`))
  (`AudioComponent.FadeIn` _spellsound 5.0 1.0 0.0 "Linear")
  (`KismetSystemLibrary.Delay` (`self.Duration`))
  (`ActorComponent.Deactivate` (`self.Niagara`))
  (`AudioComponent.FadeOut` _spellsound 5.0 0.0 "Linear"))

(event `self.SphereCol.OnComponentBeginOverlap`
  (params (OverlappedComponent :type "PrimitiveComponent Object Reference") (OtherActor :type "Actor Object Reference") (OtherComp :type "PrimitiveComponent Object Reference") (OtherBodyIndex :type Integer) (bFromSweep :type Boolean) (SweepResult :type "HitResult Structure (by ref)"))
  (bind _attackingactor (`self.AttackingActor`))
  (if (`KismetSystemLibrary.DoesImplementInterface` OtherActor "/Game/EnemyAI/AITesting/ReferenceAI/HealthDamageInterface.HealthDamageInterface_C")
    (if (not (== OtherActor _attackingactor))
      (message `/Game/EnemyAI/AITesting/ReferenceAI/HealthDamageInterface.IceStorm` OtherActor (`self.Damage`) (`self.Duration`) true _attackingactor))))

(event `self.Niagara.OnComponentDeactivated`
  (params (Component :type "ActorComponent Object Reference"))
  (`KismetSystemLibrary.Delay` 1.0)
  (`ActorComponent.Deactivate` (`self.SphereCol`))
  (`KismetSystemLibrary.Delay` 20.0)
  (`self.K2_DestroyActor`))

(fn `UserConstructionScript`)