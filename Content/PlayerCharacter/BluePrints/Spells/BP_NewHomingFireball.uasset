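; Homing fireball spell projectile that damages players or enemies on hit.
; SetHoming locks its projectile movement onto a given component, while a timeline drives homing acceleration and switches homing off when finished.
; Shortly after spawn it sets its collision sphere radius.
; On hit it spawns Niagara sparks, sends damage through HealthDamageInterface with separate player and enemy messages, makes noise via its owner and destroys itself.
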(event `self.ReceiveBeginPlay`
  (`KismetSystemLibrary.Delay` 0.2)
  (`SphereComponent.SetSphereRadius` (`self.Sphere`) 16.0 true))

(event `SetHoming`
  (params (Component :type "SceneComponent Object Reference"))
  (bind _projectilemovement (`self.ProjectileMovement`))
  (if (`KismetSystemLibrary.IsValid` Component)
    (set `ProjectileMovementComponent.bIsHomingProjectile` true _projectilemovement)
    (set `ProjectileMovementComponent.HomingAccelerationMagnitude` 10000.0 _projectilemovement)
    (set `ProjectileMovementComponent.HomingTargetComponent` Component _projectilemovement)
    (bind (_direction _newtrack_0) (`Timeline|Decrease Homing`)
      (:`Update`
        (set `ProjectileMovementComponent.HomingAccelerationMagnitude` _newtrack_0 _projectilemovement))
      (:`Finished`
        (set `ProjectileMovementComponent.bIsHomingProjectile` false _projectilemovement)))))

(event `self.ReceiveHit`
  (params (MyComp :type "PrimitiveComponent Object Reference") (Other :type "Actor Object Reference") (OtherComp :type "PrimitiveComponent Object Reference") (bSelfMoved :type Boolean) (HitLocation :type "Vector Structure") (HitNormal :type "Vector Structure") (NormalImpulse :type "Vector Structure") (Hit :type "HitResult Structure (by ref)"))
  (bind _damage (`self.Damage`))
  (set `self.HitActor` Other)
  (`NiagaraFunctionLibrary.SpawnSystemAtLocation` "/Game/VFX/NS_Sparks.NS_Sparks" HitLocation (`KismetMathLibrary.MakeRotFromZ` HitNormal))
  (if (`KismetSystemLibrary.DoesImplementInterface` (`self.HitActor`) "/Game/EnemyAI/AITesting/ReferenceAI/HealthDamageInterface.HealthDamageInterface_C")
    (bind _yes_no (message `/Game/PlayerCharacter/BluePrints/BPI_PlayerCharacter.Is Player?` (`self.HitActor`)))
    (if _yes_no
      (message `/Game/EnemyAI/AITesting/ReferenceAI/HealthDamageInterface.HitPlayer` (`self.HitActor`) _damage)
      (else
        (message `/Game/EnemyAI/AITesting/ReferenceAI/HealthDamageInterface.FireBallHitEnemy` (`self.HitActor`) _damage))))
  (`self.MakeNoise` (`self.GetOwner`) 1.0 null HitLocation (`self.NoiseRange`) "0")
  (`self.K2_DestroyActor`))

(fn `UserConstructionScript`)