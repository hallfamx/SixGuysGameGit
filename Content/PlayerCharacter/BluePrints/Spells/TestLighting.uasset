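; Lightning spell projectile that damages what it hits and shock-stuns non-player targets through HealthDamageInterface.
; SetHoming attaches a raised scene component to the target as the homing point, and Tick switches homing off once the projectile gets close.
; On hit it spawns sparks, sends player or non-player damage messages, makes noise for non-damageable hits, and destroys itself.
; Shortly after spawning, it sets its collision sphere radius.
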(event `self.ReceiveBeginPlay`
  ;[0.3542 1 0.3545] Begin Play
  (set `self.Attacking Actor` (`self.Instigator`))
  (`KismetSystemLibrary.Delay` 0.2)
  (`SphereComponent.SetSphereRadius` (`self.Sphere`) 16.0 true))

(event `self.ReceiveTick`
  (params (DeltaSeconds :type "Float (single-precision)"))
  (bind _projectilemovement (`self.ProjectileMovement`))
  ;[0.3075 0.4947 1] Homing
  (if (`ProjectileMovementComponent.bIsHomingProjectile` _projectilemovement)
    (if (< (`KismetMathLibrary.Vector_Distance` (`self.K2_GetActorLocation`) (`SceneComponent.K2_GetComponentLocation` (stale `SetHoming` _returnvalue))) 300.0)
      (set `ProjectileMovementComponent.bIsHomingProjectile` false _projectilemovement))))

(event `SetHoming`
  (params (TargetActor :type "Actor Object Reference") (MeshComponent :type "SkeletalMeshComponent Object Reference"))
  (bind (_relativelocation_x _relativelocation_y _relativelocation_z) (`KismetMathLibrary.BreakVector` (`SceneComponent.RelativeLocation` MeshComponent)))
  (bind _projectilemovement (`self.ProjectileMovement`))
  ;[0.3075 0.4947 1] Homing
  (bind _returnvalue (`AddComponent|NODE_AddSceneComponent-0` :`self` TargetActor :`RelativeTransform` (`KismetMathLibrary.MakeTransform` (`KismetMathLibrary.MakeVector` 0.0 0.0 (+ _relativelocation_z 40.0)))))
  (set `ProjectileMovementComponent.bIsHomingProjectile` true _projectilemovement)
  (set `ProjectileMovementComponent.HomingAccelerationMagnitude` 10000.0 _projectilemovement)
  (set `ProjectileMovementComponent.HomingTargetComponent` _returnvalue _projectilemovement))

(event `self.ReceiveHit`
  (params (MyComp :type "PrimitiveComponent Object Reference") (Other :type "Actor Object Reference") (OtherComp :type "PrimitiveComponent Object Reference") (bSelfMoved :type Boolean) (HitLocation :type "Vector Structure") (HitNormal :type "Vector Structure") (NormalImpulse :type "Vector Structure") (Hit :type "HitResult Structure (by ref)"))
  ;[1 0.2292 0.2292] OnHit
  (set `self.HitActor` Other)
  (`NiagaraFunctionLibrary.SpawnSystemAtLocation` "/Game/VFX/NS_Sparks.NS_Sparks" HitLocation (`KismetMathLibrary.MakeRotFromZ` HitNormal))
  (if (`KismetSystemLibrary.DoesImplementInterface` (`self.HitActor`) "/Game/EnemyAI/AITesting/ReferenceAI/HealthDamageInterface.HealthDamageInterface_C")
    (bind _yes_no (message `/Game/PlayerCharacter/BluePrints/BPI_PlayerCharacter.Is Player?` (`self.HitActor`)))
    (if _yes_no
      (message `/Game/EnemyAI/AITesting/ReferenceAI/HealthDamageInterface.GeneralHitEnemy` (`self.HitActor`) (`self.Damage`) (`self.Attacking Actor`))
      (else
        (message `/Game/EnemyAI/AITesting/ReferenceAI/HealthDamageInterface.ShockStun` (`self.HitActor`) (`self.Damage`) (`self.Duration`) (`self.Attacking Actor`))))
    (else
      (`self.MakeNoise` (`self.GetOwner`) 1.0 null HitLocation (`self.NoiseRange`) "0")))
  (`self.K2_DestroyActor`))

(fn `UserConstructionScript`)