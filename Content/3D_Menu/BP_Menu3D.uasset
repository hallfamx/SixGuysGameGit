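; BP_Menu3D is a world-placed 3D menu actor that moves the player's view between linked menus.
; On BeginPlay it binds to the transition event of its Menu3D_Widget, which passes an index into LinkedMenus.
; A transition blends the camera to the target menu with eased timing.
; Collision is disabled on the current menu and restored on the target only after a delay that outlasts the blend.
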(event `self.ReceiveBeginPlay`
  (bind _asmenu_3d_widget (cast `/Game/3D_Menu/Widgets/Menu3D_Widget` (`WidgetComponent.GetUserWidgetObject` (`self.Widget`))))
  (add `/Game/3D_Menu/Widgets/Menu3D_Widget.TransitionToLinkedMenu` _asmenu_3d_widget (delegate `OnTransitionBetweenMenus`)))

(event `OnTransitionBetweenMenus`
  (params (MenuIndex :type Integer))
  (if (`KismetArrayLibrary.Array_IsValidIndex` (`self.LinkedMenus`) MenuIndex)
    (`self.TransitionTo` (`|GetArrayItem` (`self.LinkedMenus`) MenuIndex))))

(event `TransitionTo`
  (params (`New Menu` :type "/Game/3D_Menu/BP_Menu3D Object Reference"))
  (`self.SetActorEnableCollision` false)
  (`PlayerController.SetViewTargetWithBlend` (`GameplayStatics.GetPlayerController` 0) `New Menu` 2.0 "VTBlend_EaseInOut" 2.0 false)
  (`self.SetActorEnableCollision` `New Menu` false)
  (`KismetSystemLibrary.Delay` 2.5)
  (`self.SetActorEnableCollision` `New Menu` true))

(fn `UserConstructionScript`)