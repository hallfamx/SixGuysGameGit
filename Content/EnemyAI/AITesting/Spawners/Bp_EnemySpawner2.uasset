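; Enemy spawner test actor that aims to keep a capped population of wandering Watcher AI around itself.
; Each Tick prunes dead or invalid entries from SpawnedActors, then requests a spawn while below the cap and CanSpawn is set.
; Watchers spawn at random reachable navmesh points within a fixed radius.
; Setup for valid spawns assigns team and color, tracks them, then after a delay sets AI mode and spawns their controller.
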(event `self.ReceiveTick`
  (params (DeltaSeconds :type "Float (single-precision)"))
  (for (_array_element _array_index) (`self.SpawnedActors`)
    (`/Engine/EditorBlueprintResources/StandardMacros.IsValid` _array_element
      (:`Is Valid`
        (bind _alive (`/Game/EnemyAI/AITesting/ReferenceAI/HealthDamageInterface.IsAlive` _array_element))
        (if (not _alive)
          (`KismetArrayLibrary.Array_RemoveItem` (`self.SpawnedActors`) _array_element)))
      (:`Is Not Valid`
        (`KismetArrayLibrary.Array_Remove` (`self.SpawnedActors`) _array_index))))
  (if (< (`KismetArrayLibrary.Array_Length` (`self.SpawnedActors`)) (`self.Max Actor Count`))
    (`self.SpawnActor`)))

(event `SpawnActor`
  (bind _spawnedactor (`self.SpawnedActor`))
  (bind _spawnedactor_2 (`self.SpawnedActor`))
  (if (`self.canSpawn`)
    (`|SpawnActorFromClass` "/Game/EnemyAI/AITesting/Watcher_Wandering.Watcher_Wandering_C" (`KismetMathLibrary.MakeTransform` (`NavigationSystemV1.K2_GetRandomReachablePointInRadius` (`self.K2_GetActorLocation`) 600.0 null null)) "Undefined" "OverrideRootScale" null null)
    (bind _output_get (set `self.SpawnedActor` null))
    (`/Engine/EditorBlueprintResources/StandardMacros.IsValid` _output_get
      (:`Is Valid`
        (set `/Game/EnemyAI/AITesting/MasterAI.TeamID` (`self.Team ID`) _spawnedactor)
        (`/Game/EnemyAI/AITesting/MasterAI.Change Color` _spawnedactor (`self.Enemy Color`))
        (`KismetArrayLibrary.Array_AddUnique` (`self.SpawnedActors`) _spawnedactor_2)
        (`KismetSystemLibrary.Delay` 1.0)
        (message `/Game/EnemyAI/AITesting/ReferenceAI/BPI_NPC.Update AIMode` _spawnedactor_2 (`self.AI Mode`))
        (`Pawn.SpawnDefaultController` _spawnedactor_2)))))

(fn `UserConstructionScript`)