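; BP_TestProjectile is an enemy AI test projectile that deals damage on hit.
; On BeginPlay it stores its instigator as the attacking actor and plays a spell firing sound at its location.
; On hit, it sends damage and the attacker through HealthDamageInterface to actors implementing it, then destroys itself.
; Non-damageable hits also destroy it, while hits on an interface-implementing instigator are ignored.
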(event `self.ReceiveBeginPlay`
  (set `self.AttackingActor` (`self.GetInstigator`))
  (`GameplayStatics.PlaySoundAtLocation` "/Game/PlayerCharacter/Sounds/EnemySpell.EnemySpell" (`self.K2_GetActorLocation`) (struct) 1.0 1.0 0.0 "/Game/PlayerCharacter/Sounds/EnemySpellAttenuation.EnemySpellAttenuation" null null null) ; Play firing sound
)

(event `self.ReceiveHit`
  (params (MyComp :type "PrimitiveComponent Object Reference") (Other :type "Actor Object Reference") (OtherComp :type "PrimitiveComponent Object Reference") (bSelfMoved :type Boolean) (HitLocation :type "Vector Structure") (HitNormal :type "Vector Structure") (NormalImpulse :type "Vector Structure") (Hit :type "HitResult Structure (by ref)"))
  (if (`KismetSystemLibrary.DoesImplementInterface` Other "/Game/EnemyAI/AITesting/ReferenceAI/HealthDamageInterface.HealthDamageInterface_C")
    (if (not (== (`self.AttackingActor`) Other))
      (message `/Game/EnemyAI/AITesting/ReferenceAI/HealthDamageInterface.GeneralHitEnemy` Other (`self.Damage`) (`self.AttackingActor`))
      (`self.K2_DestroyActor` :!label _label))
    (else
      (goto _label))))

(fn `UserConstructionScript`)